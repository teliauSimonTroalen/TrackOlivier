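; Conveyor belt actor that carries whatever actors overlap its Box along the forward direction of its StaticMesh.
; Every tick it gathers the overlapping actors and removes the first Landscape found and all Conveyor actors, looked up afresh each frame.
; The rest are offset in world space by Speed scaled by delta time, teleported without sweep, so the movement ignores collision.
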(event EventTick
  (params (DeltaSeconds :type Float%20%28single-precision%29))
  (bind _returnvalue (Actor|GetActorOfClass "/Script/Landscape.Landscape"))
  (bind _outactors (Actor|GetAllActorsOfClass "Conveyor_C"))
  (bind _output_get (Variables|Default|SetOverlapping%20Actors (Collision|GetOverlappingActors (Variables|Default|GetBox) 0 :!class /Script/Engine.PrimitiveComponent)))
  (Utilities|Array|RemoveItem _output_get _returnvalue)
  (for _array_element _outactors
    (Utilities|Array|RemoveItem _output_get _array_element))
  (for _array_element_2 _output_get
    (Transformation|AddActorWorldOffset _array_element_2 (* (Math|Vector|GetForwardVector (Transformation|GetWorldRotation (Variables|Default|GetStaticMesh))) (* DeltaSeconds (Variables|Default|GetSpeed))) false true)))

(fn ConstructionScript)