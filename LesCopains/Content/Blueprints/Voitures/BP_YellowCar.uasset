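; BP_YellowCar is a player car with an aimable gun that damages BP_IA_Car actors.
; Fire line-traces from the Arrow along the ChaseCamera's forward vector, with debug drawing, and applies damage on a hit.
; Turn and LookUp share one handler that applies the axis value to both yaw and inverted pitch of Scene1 and Cylinder1, clamping only the cylinder's pitch.
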(event EventBeginPlay
  (|CallParentFunction) ; This node is disabled and will not be called.\nDrag off pins to build functionality.
)

(event Collision|EventActorBeginOverlap
  (params (OtherActor :type Actor%20Object%20Reference)))

(event EventTick
  (params (DeltaSeconds :type Float%20%28single-precision%29))
  (|CallParentFunction DeltaSeconds) ; This node is disabled and will not be called.\nDrag off pins to build functionality.
)

(event Input|ActionEvents|InputActionFire
  (params (Key :type Key%20Structure :default "None"))
  (bind _arrow (Variables|Default|GetArrow))
  (bind _returnvalue (Transformation|GetWorldLocation _arrow))
  (:Pressed
    (bind (_outhit _returnvalue_2) (Collision|LineTraceByChannel _returnvalue (+ (* (Math|Vector|GetForwardVector (Variables|Default|GetChaseCamera)) (Variables|Default|GetGD_TirerLoin)) _returnvalue) "TraceTypeQuery1" false 0 "ForDuration"))
    (if _returnvalue_2
      (bind _asbp_ia_car (Utilities|Casting|CastToBP_IA_Car (.HitActor (Collision|BreakHitResult _outhit))))
      (Game|Damage|ApplyDamage _asbp_ia_car (Variables|Default|GetGD_Kaboom) 0 0))))

(event Input|AxisEvents|InputAxisLookUp
  (params (AxisValue :type Float%20%28single-precision%29))
  (bind _returnvalue (* -1 AxisValue))
  (bind _scene1 (Variables|Default|GetScene1))
  (bind _scene1_2 (Variables|Default|GetScene1))
  (bind _returnvalue_2 (Transformation|GetSocketRotation _scene1 "None"))
  (bind _returnvalue_3 (+ (.pitch _returnvalue_2) _returnvalue))
  (Transformation|SetWorldRotation _scene1_2 (Math|Rotator|MakeRotator 0.0 _returnvalue_3 (+ (.yaw (Transformation|GetSocketRotation _scene1_2 "None")) (stale Input|AxisEvents|InputAxisTurn AxisValue))) false false)
  (Transformation|SetWorldRotation (Variables|Default|GetCylinder1) (Math|Rotator|MakeRotator 0.0 (Math|Float|Clamp(Float) _returnvalue_3 -1e+01 1e+01) (+ (.yaw (Transformation|GetSocketRotation _scene1_2 "None")) (stale Input|AxisEvents|InputAxisTurn AxisValue))) false false))

(event Input|AxisEvents|InputAxisTurn
  (params (AxisValue :type Float%20%28single-precision%29))
  (bind _scene1 (Variables|Default|GetScene1))
  (bind _returnvalue (Transformation|GetSocketRotation _scene1 "None"))
  (bind _returnvalue_2 (+ (.yaw _returnvalue) AxisValue))
  (Transformation|SetWorldRotation _scene1 (Math|Rotator|MakeRotator 0.0 (+ (.pitch (Transformation|GetSocketRotation (Variables|Default|GetScene1) "None")) (* -1 (stale Input|AxisEvents|InputAxisLookUp AxisValue))) _returnvalue_2) false false)
  (Transformation|SetWorldRotation (Variables|Default|GetCylinder1) (Math|Rotator|MakeRotator 0.0 (Math|Float|Clamp(Float) (+ (.pitch (Transformation|GetSocketRotation (Variables|Default|GetScene1) "None")) (* -1 (stale Input|AxisEvents|InputAxisLookUp AxisValue))) -1e+01 1e+01) _returnvalue_2) false false))

(fn ConstructionScript
  (|CallParentFunction))