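; AI-driven car Blueprint that takes damage, shows a life widget while seen, and destroys itself at zero life.
; BeginPlay runs the BT_Car behavior tree and sets its SpeedWanted key.
; Tick spawns an explosion emitter at the blackboard's PositionCibleProche, zeroes Scene2's roll and pushes life to the widget.
; ISeeUBitch sets IsSeen to reveal the widget, and a three-second Delay driven from Tick clears it.
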(event EventBeginPlay
  (bind _self self)
  (|CallParentFunction)
  (Utilities|FlowControl|Sequence
    (:then_0
      (AI|RunBehaviorTree (AI|GetAIController _self) "/Game/Blueprints/IA/BT_Car.BT_Car")
      (bind _aslife_points_mechants (Utilities|Casting|CastToLife_Points_Mechants (UserInterface|GetUserWidgetObject (Variables|Default|GetWidget))))
      (Variables|Default|SetAs%20Life%20Points%20Mechants _aslife_points_mechants))
    (:then_1
      (AI|Components|Blackboard|SetValueasFloat (AI|GetBlackboard _self) (Utilities|Name|MakeLiteralName "SpeedWanted") 1.0))))

(event EventISeeUBitch
  (Variables|Default|SetisSeen true))

(event EventTick
  (params (DeltaSeconds :type Float%20%28single-precision%29))
  (bind _scene2 (Variables|Default|GetScene2))
  (bind _widget (Variables|Default|GetWidget))
  (bind _returnvalue (Transformation|GetWorldRotation _scene2))
  (|CallParentFunction DeltaSeconds)
  (Utilities|FlowControl|Sequence
    (:then_0
      (Effects|SpawnEmitteratLocation "/Game/StarterContent/Particles/P_Explosion.P_Explosion" (AI|Components|Blackboard|GetValueasVector (AI|GetBlackboard self) (Utilities|Name|MakeLiteralName "PositionCibleProche")))
      (Transformation|SetWorldRotation _scene2 (Math|Rotator|MakeRotator 0.0 (.pitch _returnvalue) (.yaw _returnvalue)) false false))
    (:then_1
      (Utilities|FlowControl|Sequence
        (:then_0
          (Utilities|FlowControl|Delay 3.0)
          (Variables|Default|SetisSeen false))
        (:then_1
          (if (Variables|Default|GetisSeen)
            (Rendering|SetVisibility _widget true false)
            (else
              (Rendering|SetVisibility _widget false false))))
        (:then_2
          (Variables|/Game/Blueprints/UI/Life_Points_Mechants.Life_Points_Mechants_C|Setlifepoint (Variables|Default|GetAs%20Life%20Points%20Mechants) (Variables|Default|GetLIFEPOINT)))))))

(event Game|Damage|EventAnyDamage
  (params (Damage :type Float%20%28single-precision%29) (DamageType :type Damage%20Type%20Object%20Reference) (InstigatedBy :type Controller%20Object%20Reference) (DamageCauser :type Actor%20Object%20Reference))
  (Variables|Default|SetLIFEPOINT (- (Variables|Default|GetLIFEPOINT) Damage))
  (if (<= (Variables|Default|GetLIFEPOINT) 0.0)
    (Actor|DestroyActor)))

(event Collision|EventActorBeginOverlap
  (params (OtherActor :type Actor%20Object%20Reference)))

(fn ConstructionScript
  (|CallParentFunction))