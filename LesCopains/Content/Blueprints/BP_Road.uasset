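; BP_Road is a spline-based road Blueprint that so far holds only placeholder or debug logic.
; On BeginPlay it resets Indentation to zero, then loops up to the truncated spline length, printing each index.
; Nodes for adding spline points and sampling locations by distance are present but unconnected, and the construction script is empty, so no road geometry is built.
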(event EventBeginPlay
  (Variables|Default|SetIndentation 0)
  (for _index (range (Variables|Default|GetIndentation) (Math|Float|Truncate (Spline|GetSplineLength (Variables|Default|GetSpline))))
    (Development|PrintString (Utilities|String|ToString(Integer) _index))))

(fn ConstructionScript)