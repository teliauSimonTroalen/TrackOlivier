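; Behavior Tree task that steers a BP_IA_Car along the BP_Road spline.
; It projects the car's Mid point onto the spline and picks near and far targets with speed-scaled look-ahead.
; LP/RP distance differences give direction and speed-damped turn rate, offset by blackboard ViragePoulpe, for Turn.
; It writes both targets, TurnRate and far-bend VirageRating to the blackboard; without a road it only prints, never finishing.
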(event EventReceiveExecuteAI
  (params (OwnerController :type AI%20Controller%20Object%20Reference) (ControlledPawn :type Pawn%20Object%20Reference))
  (bind _returnvalue (Transformation|GetVelocity ControlledPawn))
  (bind _returnvalue_2 (Math|Vector|VectorLength _returnvalue))
  (bind _asbp_ia_car (Utilities|Casting|CastToBP_IA_Car ControlledPawn))
  (bind _returnvalue_3 (Actor|GetActorOfClass "/Game/Blueprints/BP_Road.BP_Road_C"))
  (Utilities|IsValid _returnvalue_3
    (:Is%20Valid
      (bind _distance (CallFunction|FromPositiontoDistance (Variables|/Game/Blueprints/BP_Road.BP_Road_C|GetSpline _returnvalue_3) (Spline|FindLocationClosesttoWorldLocation (Variables|/Game/Blueprints/BP_Road.BP_Road_C|GetSpline _returnvalue_3) (Transformation|GetWorldLocation (Variables|/Game/Blueprints/BP_IA_Car.BP_IA_Car_C|GetMid _asbp_ia_car)) "World")))
      (bind _distance_2 (CallFunction|FromPositiontoDistance (Variables|/Game/Blueprints/BP_Road.BP_Road_C|GetSpline _returnvalue_3) (Spline|FindLocationClosesttoWorldLocation (Variables|/Game/Blueprints/BP_Road.BP_Road_C|GetSpline _returnvalue_3) (Transformation|GetWorldLocation (Variables|/Game/Blueprints/BP_IA_Car.BP_IA_Car_C|GetMid _asbp_ia_car)) "World")))
      (AI|Components|Blackboard|SetValueasFloat (AI|GetBlackboard _asbp_ia_car) (Utilities|Name|MakeLiteralName "VirageRating") (/ (Math|Float|Absolute(Float) (- (Math|Vector|Distance(Vector) (Spline|GetLocationatDistanceAlongSpline (Variables|/Game/Blueprints/BP_Road.BP_Road_C|GetSpline _returnvalue_3) (+ _distance_2 (* _returnvalue_2 4.5) 0.0) "World") (Transformation|GetWorldLocation (Variables|/Game/Blueprints/BP_IA_Car.BP_IA_Car_C|GetLP _asbp_ia_car))) (Math|Vector|Distance(Vector) (Spline|GetLocationatDistanceAlongSpline (Variables|/Game/Blueprints/BP_Road.BP_Road_C|GetSpline _returnvalue_3) (+ _distance_2 (* _returnvalue_2 4.5) 0.0) "World") (Transformation|GetWorldLocation (Variables|/Game/Blueprints/BP_IA_Car.BP_IA_Car_C|GetRP _asbp_ia_car))))) 1.8e+02))
      (AI|Components|Blackboard|SetValueasVector (AI|GetBlackboard _asbp_ia_car) (Utilities|Name|MakeLiteralName "PositionCibleProche") (Spline|GetLocationatDistanceAlongSpline (Variables|/Game/Blueprints/BP_Road.BP_Road_C|GetSpline _returnvalue_3) (+ _distance (* _returnvalue_2 3.0) 1e+01) "World"))
      (AI|Components|Blackboard|SetValueasVector (AI|GetBlackboard _asbp_ia_car) (Utilities|Name|MakeLiteralName "PositionCibleLointaine") (Spline|GetLocationatDistanceAlongSpline (Variables|/Game/Blueprints/BP_Road.BP_Road_C|GetSpline _returnvalue_3) (+ _distance_2 (* _returnvalue_2 4.5) 0.0) "World"))
      (AI|Components|Blackboard|SetValueasFloat (AI|GetBlackboard _asbp_ia_car) (Utilities|Name|MakeLiteralName "TurnRate") (/ (Math|Float|Absolute(Float) (- (Math|Vector|Distance(Vector) (Spline|GetLocationatDistanceAlongSpline (Variables|/Game/Blueprints/BP_Road.BP_Road_C|GetSpline _returnvalue_3) (+ _distance (* _returnvalue_2 3.0) 1e+01) "World") (Transformation|GetWorldLocation (Variables|/Game/Blueprints/BP_IA_Car.BP_IA_Car_C|GetLP _asbp_ia_car))) (Math|Vector|Distance(Vector) (Spline|GetLocationatDistanceAlongSpline (Variables|/Game/Blueprints/BP_Road.BP_Road_C|GetSpline _returnvalue_3) (+ _distance (* _returnvalue_2 3.0) 1e+01) "World") (Transformation|GetWorldLocation (Variables|/Game/Blueprints/BP_IA_Car.BP_IA_Car_C|GetRP _asbp_ia_car))))) (* (Math|Float|Clamp(Float) (* (Math|Vector|VectorLength (Transformation|GetVelocity ControlledPawn)) 0.0005) 1.0 9999999.0) 1.8e+02)))
      (if (< (Math|Vector|Distance(Vector) (Spline|GetLocationatDistanceAlongSpline (Variables|/Game/Blueprints/BP_Road.BP_Road_C|GetSpline _returnvalue_3) (+ _distance (* _returnvalue_2 3.0) 1e+01) "World") (Transformation|GetWorldLocation (Variables|/Game/Blueprints/BP_IA_Car.BP_IA_Car_C|GetLP _asbp_ia_car))) (Math|Vector|Distance(Vector) (Spline|GetLocationatDistanceAlongSpline (Variables|/Game/Blueprints/BP_Road.BP_Road_C|GetSpline _returnvalue_3) (+ _distance (* _returnvalue_2 3.0) 1e+01) "World") (Transformation|GetWorldLocation (Variables|/Game/Blueprints/BP_IA_Car.BP_IA_Car_C|GetRP _asbp_ia_car))))
        (Default|Turn _asbp_ia_car (+ (* -1 (/ (Math|Float|Absolute(Float) (- (Math|Vector|Distance(Vector) (Spline|GetLocationatDistanceAlongSpline (Variables|/Game/Blueprints/BP_Road.BP_Road_C|GetSpline _returnvalue_3) (+ _distance (* _returnvalue_2 3.0) 1e+01) "World") (Transformation|GetWorldLocation (Variables|/Game/Blueprints/BP_IA_Car.BP_IA_Car_C|GetLP _asbp_ia_car))) (Math|Vector|Distance(Vector) (Spline|GetLocationatDistanceAlongSpline (Variables|/Game/Blueprints/BP_Road.BP_Road_C|GetSpline _returnvalue_3) (+ _distance (* _returnvalue_2 3.0) 1e+01) "World") (Transformation|GetWorldLocation (Variables|/Game/Blueprints/BP_IA_Car.BP_IA_Car_C|GetRP _asbp_ia_car))))) (* (Math|Float|Clamp(Float) (* (Math|Vector|VectorLength (Transformation|GetVelocity ControlledPawn)) 0.0005) 1.0 9999999.0) 1.8e+02))) (Class|BlackboardComponent|GetValueasFloat (AI|GetBlackboard _asbp_ia_car) (Utilities|Name|MakeLiteralName "ViragePoulpe"))))
        (else
          (Default|Turn _asbp_ia_car (+ (/ (Math|Float|Absolute(Float) (- (Math|Vector|Distance(Vector) (Spline|GetLocationatDistanceAlongSpline (Variables|/Game/Blueprints/BP_Road.BP_Road_C|GetSpline _returnvalue_3) (+ _distance (* _returnvalue_2 3.0) 1e+01) "World") (Transformation|GetWorldLocation (Variables|/Game/Blueprints/BP_IA_Car.BP_IA_Car_C|GetLP _asbp_ia_car))) (Math|Vector|Distance(Vector) (Spline|GetLocationatDistanceAlongSpline (Variables|/Game/Blueprints/BP_Road.BP_Road_C|GetSpline _returnvalue_3) (+ _distance (* _returnvalue_2 3.0) 1e+01) "World") (Transformation|GetWorldLocation (Variables|/Game/Blueprints/BP_IA_Car.BP_IA_Car_C|GetRP _asbp_ia_car))))) (* (Math|Float|Clamp(Float) (* (Math|Vector|VectorLength (Transformation|GetVelocity ControlledPawn)) 0.0005) 1.0 9999999.0) 1.8e+02)) (Class|BlackboardComponent|GetValueasFloat (AI|GetBlackboard _asbp_ia_car) (Utilities|Name|MakeLiteralName "ViragePoulpe"))))))
      (AI|BehaviorTree|FinishExecute true))
    (:Is%20Not%20Valid
      (Development|PrintString "Mettez un BP_Road bande de débiles"))))

(fn FromPositiontoDistance
  (params (Spline :type Spline%20Component%20Object%20Reference) (Position :type Vector))
  (bind _returnvalue (Class|SplineComponent|FindInputKeyClosesttoWorldLocation Spline Position))
  (bind _returnvalue_2 (Math|Float|Truncate _returnvalue))
  (bind _returnvalue_3 (Spline|GetDistanceAlongSplineatSplinePoint Spline _returnvalue_2))
  (return (+ _returnvalue_3 (* (- (Spline|GetDistanceAlongSplineatSplinePoint Spline (Math|Float|Truncate (+ _returnvalue 1.0))) _returnvalue_3) (- _returnvalue (Math|Conversions|ToFloat(Integer) _returnvalue_2))))))