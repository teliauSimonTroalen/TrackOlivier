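; Behavior Tree service that sets the throttle target for AI cars (BP_IA_Car) each time it activates.
; It compares the blackboard VirageRating (turn rating) and the car's velocity against two thresholds, giving four cases.
; Each case scales and clamps the SpeedWanted blackboard value: gradual changes at low turn rating, a stronger cut at high rating, and a damped sign flip when also fast.
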(event EventReceiveActivationAI
  (params (OwnerController :type AI%20Controller%20Object%20Reference) (ControlledPawn :type Pawn%20Object%20Reference))
  (bind _returnvalue (AI|GetBlackboard OwnerController))
  (bind _returnvalue_2 (Utilities|Name|MakeLiteralName "SpeedWanted"))
  (bind _returnvalue_3 (Utilities|Name|MakeLiteralName "VirageRating"))
  (bind _returnvalue_4 (Class|BlackboardComponent|GetValueasFloat _returnvalue _returnvalue_2))
  (bind _returnvalue_5 (Class|BlackboardComponent|GetValueasFloat _returnvalue _returnvalue_3))
  (bind _asbp_ia_car (Utilities|Casting|CastToBP_IA_Car ControlledPawn))
  (if (and (< _returnvalue_5 (Variables|Default|GetSeuilTournage)) (< (Math|Vector|VectorLength (Transformation|GetVelocity _asbp_ia_car)) (Variables|Default|GetSeuilSpeed)))
    (Variables|Default|SetCas 0))
  (if (and (< _returnvalue_5 (Variables|Default|GetSeuilTournage)) (> (Math|Vector|VectorLength (Transformation|GetVelocity _asbp_ia_car)) (Variables|Default|GetSeuilSpeed)))
    (Variables|Default|SetCas 1))
  (if (and (> _returnvalue_5 (Variables|Default|GetSeuilTournage)) (< (Math|Vector|VectorLength (Transformation|GetVelocity _asbp_ia_car)) (Variables|Default|GetSeuilSpeed)))
    (Variables|Default|SetCas 2))
  (if (and (> _returnvalue_5 (Variables|Default|GetSeuilTournage)) (> (Math|Vector|VectorLength (Transformation|GetVelocity _asbp_ia_car)) (Variables|Default|GetSeuilSpeed)))
    (Variables|Default|SetCas 3))
  (switch int (Variables|Default|GetCas)
    (:0
      (AI|Components|Blackboard|SetValueasFloat _returnvalue _returnvalue_2 (Math|Float|Clamp(Float) (* _returnvalue_4 1.01) 0.7)))
    (:1
      (AI|Components|Blackboard|SetValueasFloat _returnvalue _returnvalue_2 (Math|Float|Clamp(Float) (* _returnvalue_4 0.99) 0.4)))
    (:2
      (AI|Components|Blackboard|SetValueasFloat _returnvalue _returnvalue_2 (Math|Float|Clamp(Float) (* _returnvalue_4 0.7) 0.4 0.6)))
    (:3
      (AI|Components|Blackboard|SetValueasFloat _returnvalue _returnvalue_2 (Math|Float|Clamp(Float) (* _returnvalue_4 -0.1) -1.0)))))