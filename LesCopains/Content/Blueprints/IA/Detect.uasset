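; Behavior tree task for the AI car that casts forward sensor rays from the controlled BP_IA_Car pawn.
; A sequence fires five line traces on the Camera channel, 1000 units along the car's left-to-right arrow components, with debug draw.
; Trace results are not read, and each branch calls FinishExecute with success.
; A failed pawn cast stops the task without finishing it.
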(event EventReceiveExecuteAI
  (params (OwnerController :type AI%20Controller%20Object%20Reference) (ControlledPawn :type Pawn%20Object%20Reference))
  (bind _draw_debug_type (Variables|Default|GetDraw%20Debug%20Type))
  (bind _asbp_ia_car (Utilities|Casting|CastToBP_IA_Car ControlledPawn))
  (Utilities|FlowControl|Sequence
    (:then_0
      (Collision|LineTraceByChannel (Transformation|GetWorldLocation (Variables|/Game/Blueprints/BP_IA_Car.BP_IA_Car_C|GetArrowLeftLeft _asbp_ia_car)) (+ (Transformation|GetWorldLocation (Variables|/Game/Blueprints/BP_IA_Car.BP_IA_Car_C|GetArrowLeftLeft _asbp_ia_car)) (* (Math|Vector|GetForwardVector (Transformation|GetWorldRotation (Variables|/Game/Blueprints/BP_IA_Car.BP_IA_Car_C|GetArrowLeftLeft _asbp_ia_car))) 1e+03)) "TraceTypeQuery2" false 0 _draw_debug_type))
    (:then_1
      (Collision|LineTraceByChannel (Transformation|GetWorldLocation (Variables|/Game/Blueprints/BP_IA_Car.BP_IA_Car_C|GetArrowLeft _asbp_ia_car)) (+ (* (Math|Vector|GetForwardVector (Transformation|GetWorldRotation (Variables|/Game/Blueprints/BP_IA_Car.BP_IA_Car_C|GetArrowLeft _asbp_ia_car))) 1e+03) (Transformation|GetWorldLocation (Variables|/Game/Blueprints/BP_IA_Car.BP_IA_Car_C|GetArrowLeft _asbp_ia_car))) "TraceTypeQuery2" false 0 _draw_debug_type))
    (:then_2
      (Collision|LineTraceByChannel (Transformation|GetWorldLocation (Variables|/Game/Blueprints/BP_IA_Car.BP_IA_Car_C|GetArrowMid _asbp_ia_car)) (+ (Transformation|GetWorldLocation (Variables|/Game/Blueprints/BP_IA_Car.BP_IA_Car_C|GetArrowMid _asbp_ia_car)) (* (Math|Vector|GetForwardVector (Transformation|GetWorldRotation (Variables|/Game/Blueprints/BP_IA_Car.BP_IA_Car_C|GetArrowMid _asbp_ia_car))) 1e+03)) "TraceTypeQuery2" false 0 _draw_debug_type))
    (:then_3
      (Collision|LineTraceByChannel (Transformation|GetWorldLocation (Variables|/Game/Blueprints/BP_IA_Car.BP_IA_Car_C|GetArrowRight _asbp_ia_car)) (+ (Transformation|GetWorldLocation (Variables|/Game/Blueprints/BP_IA_Car.BP_IA_Car_C|GetArrowRight _asbp_ia_car)) (* (Math|Vector|GetForwardVector (Transformation|GetWorldRotation (Variables|/Game/Blueprints/BP_IA_Car.BP_IA_Car_C|GetArrowRight _asbp_ia_car))) 1e+03)) "TraceTypeQuery2" false 0 _draw_debug_type))
    (:then_4
      (Collision|LineTraceByChannel (Transformation|GetWorldLocation (Variables|/Game/Blueprints/BP_IA_Car.BP_IA_Car_C|GetArrowRightRight _asbp_ia_car)) (+ (Transformation|GetWorldLocation (Variables|/Game/Blueprints/BP_IA_Car.BP_IA_Car_C|GetArrowRightRight _asbp_ia_car)) (* (Math|Vector|GetForwardVector (Transformation|GetWorldRotation (Variables|/Game/Blueprints/BP_IA_Car.BP_IA_Car_C|GetArrowRightRight _asbp_ia_car))) 1e+03)) "TraceTypeQuery2" false 0 _draw_debug_type true "(R=1.000000,G=0.000000,B=0.000000,A=1.000000)" "(R=0.000000,G=1.000000,B=0.000000,A=1.000000)" 1.0)))
  (AI|BehaviorTree|FinishExecute true))