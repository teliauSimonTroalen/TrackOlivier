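; LePoulpe is a Behavior Tree service that steers a BP_IA_Car away from obstacles whenever the service activates.
; It fires five Camera-channel line traces from the car's arrow components, fanned left to right.
; Each hit adds a side-specific bias to OnTourne (random for the middle), which is never reset here, and immediately calls Turn.
; If all five traces report hits, it calls Accelerate(-1) instead.
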(event EventReceiveActivationAI
  (params (OwnerController :type AI%20Controller%20Object%20Reference) (ControlledPawn :type Pawn%20Object%20Reference))
  (bind _array (Utilities|Array|MakeArray ControlledPawn 0))
  (bind _draw_debug_type (Variables|Default|GetDraw%20Debug%20Type))
  (bind _je_vois_loin (Variables|Default|GetJe%20vois%20Loin))
  (bind _asbp_ia_car (Utilities|Casting|CastToBP_IA_Car ControlledPawn))
  (Utilities|FlowControl|Sequence
    (:then_0
      (bind _returnvalue (Collision|LineTraceByChannel (Transformation|GetWorldLocation (Variables|/Game/Blueprints/BP_IA_Car.BP_IA_Car_C|GetArrowLeftLeft _asbp_ia_car)) (+ (Transformation|GetWorldLocation (Variables|/Game/Blueprints/BP_IA_Car.BP_IA_Car_C|GetArrowLeftLeft _asbp_ia_car)) (* (Math|Vector|GetForwardVector (Transformation|GetWorldRotation (Variables|/Game/Blueprints/BP_IA_Car.BP_IA_Car_C|GetArrowLeftLeft _asbp_ia_car))) _je_vois_loin)) "TraceTypeQuery2" false _array _draw_debug_type))
      (if _returnvalue
        (Variables|Default|SetOnTourne (+ (Variables|Default|GetOnTourne) 0.3))
        (if (Math|Boolean|ANDBoolean (stale _returnvalue_2) _returnvalue (stale _returnvalue_3) (stale _returnvalue_4) (stale _returnvalue_5)) :!label _label
          (Default|Accelerate _asbp_ia_car -1.0)
          (else
            (Default|Turn _asbp_ia_car (Variables|Default|GetOnTourne))))))
    (:then_1
      (bind _returnvalue_2 (Collision|LineTraceByChannel (Transformation|GetWorldLocation (Variables|/Game/Blueprints/BP_IA_Car.BP_IA_Car_C|GetArrowLeft _asbp_ia_car)) (+ (* (Math|Vector|GetForwardVector (Transformation|GetWorldRotation (Variables|/Game/Blueprints/BP_IA_Car.BP_IA_Car_C|GetArrowLeft _asbp_ia_car))) _je_vois_loin) (Transformation|GetWorldLocation (Variables|/Game/Blueprints/BP_IA_Car.BP_IA_Car_C|GetArrowLeft _asbp_ia_car))) "TraceTypeQuery2" false _array _draw_debug_type))
      (if _returnvalue_2
        (Variables|Default|SetOnTourne (+ (Variables|Default|GetOnTourne) 0.4))
        (goto _label)))
    (:then_2
      (bind _returnvalue_3 (Collision|LineTraceByChannel (Transformation|GetWorldLocation (Variables|/Game/Blueprints/BP_IA_Car.BP_IA_Car_C|GetArrowMid _asbp_ia_car)) (+ (Transformation|GetWorldLocation (Variables|/Game/Blueprints/BP_IA_Car.BP_IA_Car_C|GetArrowMid _asbp_ia_car)) (* (Math|Vector|GetForwardVector (Transformation|GetWorldRotation (Variables|/Game/Blueprints/BP_IA_Car.BP_IA_Car_C|GetArrowMid _asbp_ia_car))) 1e+03)) "TraceTypeQuery2" false _array _draw_debug_type))
      (if _returnvalue_3
        (Variables|Default|SetOnTourne (+ (Variables|Default|GetOnTourne) (* (Math|Random|RandomIntegerinRange -1 1) 0.5)))
        (goto _label)))
    (:then_3
      (bind _returnvalue_4 (Collision|LineTraceByChannel (Transformation|GetWorldLocation (Variables|/Game/Blueprints/BP_IA_Car.BP_IA_Car_C|GetArrowRight _asbp_ia_car)) (+ (Transformation|GetWorldLocation (Variables|/Game/Blueprints/BP_IA_Car.BP_IA_Car_C|GetArrowRight _asbp_ia_car)) (* (Math|Vector|GetForwardVector (Transformation|GetWorldRotation (Variables|/Game/Blueprints/BP_IA_Car.BP_IA_Car_C|GetArrowRight _asbp_ia_car))) _je_vois_loin)) "TraceTypeQuery2" false _array _draw_debug_type))
      (if _returnvalue_4
        (Variables|Default|SetOnTourne (+ (Variables|Default|GetOnTourne) -0.4))
        (goto _label)))
    (:then_4
      (bind _returnvalue_5 (Collision|LineTraceByChannel (Transformation|GetWorldLocation (Variables|/Game/Blueprints/BP_IA_Car.BP_IA_Car_C|GetArrowRightRight _asbp_ia_car)) (+ (Transformation|GetWorldLocation (Variables|/Game/Blueprints/BP_IA_Car.BP_IA_Car_C|GetArrowRightRight _asbp_ia_car)) (* (Math|Vector|GetForwardVector (Transformation|GetWorldRotation (Variables|/Game/Blueprints/BP_IA_Car.BP_IA_Car_C|GetArrowRightRight _asbp_ia_car))) _je_vois_loin)) "TraceTypeQuery2" false _array _draw_debug_type true "(R=1.000000,G=0.000000,B=0.000000,A=1.000000)" "(R=0.000000,G=1.000000,B=0.000000,A=1.000000)" 1.0))
      (if _returnvalue_5
        (Variables|Default|SetOnTourne (+ (Variables|Default|GetOnTourne) -0.2))
        (goto _label)))))