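; AI-driven car that runs the BT_Car behavior tree and carries a life-points widget.
; Tick writes its distance to the blackboard target position, flags "Is on Road" when close, and spawns an explosion emitter at that target every frame.
; The widget shows while IsSeen is set, which a repeating Delay clears, and mirrors LIFEPOINT.
; AnyDamage lowers LIFEPOINT and prints it while positive, with no death handling here.
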(event EventBeginPlay
  (bind _self self)
  (|CallParentFunction)
  (Utilities|FlowControl|Sequence
    (:then_0
      (AI|RunBehaviorTree (AI|GetAIController _self) "/Game/Blueprints/IA/BT_Car.BT_Car")
      (AI|Components|Blackboard|SetValueasFloat (AI|GetBlackboard _self) (Utilities|Name|MakeLiteralName "VitesseVroomVroom") 1.0)
      (bind _aslife_points_mechants (Utilities|Casting|CastToLife_Points_Mechants (UserInterface|GetUserWidgetObject (Variables|Default|GetWidget))))
      (Variables|Default|SetAs%20Life%20Points%20Mechants _aslife_points_mechants))))

(event EventTick
  (params (DeltaSeconds :type Float%20%28single-precision%29))
  (bind _returnvalue (Utilities|Name|MakeLiteralName "DistanceALaRoute"))
  (bind _returnvalue_2 (Utilities|Name|MakeLiteralName "Is on Road"))
  (bind _returnvalue_3 (Utilities|Name|MakeLiteralName "PositionCible"))
  (bind _self self)
  (bind _widget (Variables|Default|GetWidget))
  (bind _returnvalue_4 (AI|GetBlackboard _self))
  (bind _returnvalue_5 (AI|Components|Blackboard|GetValueasVector _returnvalue_4 _returnvalue_3))
  (|CallParentFunction DeltaSeconds)
  (Utilities|FlowControl|Sequence
    (:then_0
      (AI|Components|Blackboard|SetValueasFloat _returnvalue_4 _returnvalue (Math|Vector|Distance(Vector) (Transformation|GetWorldLocation (Variables|Default|GetMid _self)) _returnvalue_5)))
    (:then_1
      (Effects|SpawnEmitteratLocation "/Game/StarterContent/Particles/P_Explosion.P_Explosion" _returnvalue_5)
      (if (< (Class|BlackboardComponent|GetValueasFloat _returnvalue_4 _returnvalue) 2e+02)
        (AI|Components|Blackboard|SetValueasBool _returnvalue_4 _returnvalue_2 true)
        (else
          (AI|Components|Blackboard|SetValueasBool _returnvalue_4 _returnvalue_2 false))))
    (:then_2
      ;[1 1 1] Event Tick
      (Utilities|FlowControl|Sequence
        (:then_0
          (Utilities|FlowControl|Delay 3.0)
          (Variables|Default|SetisSeen false))
        (:then_1
          (if (Variables|Default|GetisSeen)
            (Rendering|SetVisibility _widget true false)
            (else
              (Rendering|SetVisibility _widget false false))))
        (:then_2
          (Variables|/Game/Blueprints/UI/Life_Points_Mechants.Life_Points_Mechants_C|Setlifepoint (Variables|Default|GetAs%20Life%20Points%20Mechants) (Variables|Default|GetLIFEPOINT)))))))

(event Game|Damage|EventAnyDamage
  (params (Damage :type Float%20%28single-precision%29) (DamageType :type Damage%20Type%20Object%20Reference) (InstigatedBy :type Controller%20Object%20Reference) (DamageCauser :type Actor%20Object%20Reference))
  (Variables|Default|SetLIFEPOINT (- (Variables|Default|GetLIFEPOINT) Damage))
  (if (not (<= (Variables|Default|GetLIFEPOINT) 0.0))
    (Development|PrintString (Utilities|String|ToString(Float) (Variables|Default|GetLIFEPOINT)))))

(event EventISeeUBitch)

(event Collision|EventActorBeginOverlap
  (params (OtherActor :type Actor%20Object%20Reference)))

(fn ConstructionScript
  (|CallParentFunction))